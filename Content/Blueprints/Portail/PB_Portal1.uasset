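; Portal actor linked to a TargetCam actor, mirroring the player's view there and teleporting actors that hit it.
; Each tick, CamTarget follows the player camera, and its relative transform is copied onto TargetCam's CamRenderer, keeping the view portal-relative.
; Hits move the other actor to that renderer's transform, with an X offset and fixed Z drop.
; The construction script adds a spline reaching to TargetCam.
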(event `self.ReceiveTick`
  (params (DeltaSeconds :type "Float (single-precision)"))
  (bind _camtarget (`self.CamTarget`))
  (bind _transformcomponent (`PlayerCameraManager.TransformComponent` (`GameplayStatics.GetPlayerCameraManager` 0)))
  (`SceneComponent.K2_SetWorldLocationAndRotation` (`self.CamTarget`) (`SceneComponent.K2_GetComponentLocation` _transformcomponent) (`SceneComponent.K2_GetComponentRotation` _transformcomponent) false false)
  (`SceneComponent.K2_SetRelativeLocationAndRotation` (`/Game/Blueprints/Portail/BP_TargetCam.CamRenderer` (`self.TargetCam`)) (`SceneComponent.RelativeLocation` _camtarget) (`SceneComponent.RelativeRotation` _camtarget) false false))

(event `self.Portal.OnComponentHit`
  (params (HitComponent :type "PrimitiveComponent Object Reference") (OtherActor :type "Actor Object Reference") (OtherComp :type "PrimitiveComponent Object Reference") (NormalImpulse :type "Vector Structure") (Hit :type "HitResult Structure (by ref)"))
  (bind _rootcomponent (`Actor.RootComponent` OtherActor))
  (bind _camrenderer (`/Game/Blueprints/Portail/BP_TargetCam.CamRenderer` (`self.TargetCam`)))
  (bind (_returnvalue_x _returnvalue_y _returnvalue_z) (`KismetMathLibrary.BreakVector` (`SceneComponent.K2_GetComponentLocation` _camrenderer)))
  (`SceneComponent.K2_SetWorldLocation` _rootcomponent (`KismetMathLibrary.MakeVector` (+ (`self.OffsetTP`) _returnvalue_x) _returnvalue_y (+ _returnvalue_z -151.327179)) false false)
  (`SceneComponent.K2_SetWorldRotation` _rootcomponent (`SceneComponent.K2_GetComponentRotation` _camrenderer) false false))

(fn `UserConstructionScript`
  (bind _targetcam (`self.TargetCam`)
    (:`then`
      (bind _returnvalue (`AddComponent|NODE_AddSplineComponent-0`))
      (`SplineComponent.SetLocationAtSplinePoint` _returnvalue 1 (`SceneComponent.K2_GetComponentLocation` (`/Game/Blueprints/Portail/BP_TargetCam.DefaultSceneRoot` _targetcam)) "World" true))
    (:`else`)))