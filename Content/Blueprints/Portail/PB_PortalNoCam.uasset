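; PB_PortalNoCam is a one-way portal that teleports any actor entering its Box to a linked TargetCam.
; On overlap, the actor's root moves to the target's CamRenderer location, shifted by OffsetTP along world X, and takes that component's rotation.
; When TargetCam is valid, the construction script adds a spline with point 1 at the target's root, linking the two.
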(event `self.Box.OnComponentBeginOverlap`
  (params (OverlappedComponent :type "PrimitiveComponent Object Reference") (OtherActor :type "Actor Object Reference") (OtherComp :type "PrimitiveComponent Object Reference") (OtherBodyIndex :type Integer) (bFromSweep :type Boolean) (SweepResult :type "HitResult Structure (by ref)"))
  (bind _rootcomponent (`Actor.RootComponent` OtherActor))
  (bind _camrenderer (`/Game/Blueprints/Portail/BP_TargetCam.CamRenderer` (`self.TargetCam`)))
  (bind (_returnvalue_x _returnvalue_y _returnvalue_z) (`KismetMathLibrary.BreakVector` (`SceneComponent.K2_GetComponentLocation` _camrenderer)))
  (`SceneComponent.K2_SetWorldLocation` _rootcomponent (`KismetMathLibrary.MakeVector` (+ (`self.OffsetTP`) _returnvalue_x) _returnvalue_y (+ _returnvalue_z 0.0)) false false)
  (`SceneComponent.K2_SetWorldRotation` _rootcomponent (`SceneComponent.K2_GetComponentRotation` _camrenderer) false false))

(fn `UserConstructionScript`
  (bind _targetcam (`self.TargetCam`)
    (:`then`
      (bind _returnvalue (`AddComponent|NODE_AddSplineComponent-0`))
      (`SplineComponent.SetLocationAtSplinePoint` _returnvalue 1 (`SceneComponent.K2_GetComponentLocation` (`/Game/Blueprints/Portail/BP_TargetCam.DefaultSceneRoot` _targetcam)) "World" true))
    (:`else`)))